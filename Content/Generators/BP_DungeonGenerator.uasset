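; BP_DungeonGenerator is a procedural dungeon generator that currently builds only the first room's floor, despite looping over a room count.
; The construction script seeds a random stream, then runs GenerateMap.
; RoomMakeFloorArea creates a randomly sized rectangle of integer grid tiles and returns it with location and extents to record.
; SpawnTiles scales those coordinates into local-space instances on the Floor component.
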(event `GenerateMap`
  (for _index (range (`self.RoomNum`))
    (if (== _index 0)
      (bind (_floortiles _location_ _extents) (`self.Room_MakeFloorArea` (`self.PrevLocation`)))
      (set `self.FloorTiles` _floortiles)
      (`BlueprintMapLibrary.Map_Add` (`self.Rooms`) _location_ _extents)))
  (`self.SpawnTiles`))

(fn `Room_MakeFloorArea`
  (params (Location :type "IntVector Structure"))
  (returns (FloorTiles :type "Array of IntVector Structure") (`Location ` :type "IntVector Structure") (Extents :type "IntVector Structure"))
  (locals (RootLocation :type "IntVector Structure") (RoomX :type Integer :default 0) (RoomY :type Integer :default 0) (Working :type Boolean :default true) (Tiles :type "Array of IntVector Structure") (ConnectedTIles :type "Array of IntVector Structure") (Extent_X :type "Array of Integer") (Extent_Y :type "Array of Integer"))
  (bind _roomsize_max (`self.RoomSize_Max`))
  (bind _roomsize_min (`self.RoomSize_Min`))
  (bind _stream (`self.Stream`))
  (bind _roomy (`local.RoomY`))
  (bind (_x _y _z) (break `IntVector` (`local.RootLocation`)))
  ;[1 1 1] Get random X and Y values
  (set `local.RootLocation` Location)
  (set `local.RoomY` (`KismetMathLibrary.RandomIntegerInRangeFromStream` _roomsize_min _roomsize_max _stream))
  (set `local.RoomX` (`KismetMathLibrary.RandomIntegerInRangeFromStream` _roomsize_min _roomsize_max _stream))
  (for _index (range (* (`local.RoomX`) (`local.RoomY`)))
    (`KismetArrayLibrary.Array_Add` (`local.Tiles`) (make `IntVector` (+ (/ _index _roomy) _x) (+ (mod _index _roomy) _y) _z)))
  (while (`local.Working`)
    (set `local.Working` false)
    (set `local.ConnectedTIles` (`local.Tiles`)))
  (for _array_element (`local.ConnectedTIles`)
    (bind (_x_2 _y_2) (break `IntVector` _array_element))
    (`KismetArrayLibrary.Array_Add` (`local.Extent_X`) _x_2)
    (`KismetArrayLibrary.Array_Add` (`local.Extent_Y`) _y_2))
  (return (`local.ConnectedTIles`) (`local.RootLocation`) (make `IntVector` (`.MaxValue` (`KismetMathLibrary.MaxOfIntArray` (`local.Extent_X`))) (`KismetMathLibrary.MaxOfIntArray` (`local.Extent_Y`)))))

(fn `SpawnTiles`
  (for _array_element (`self.FloorTiles`)
    (`InstancedStaticMeshComponent.AddInstance` (`self.Floor`) (`KismetMathLibrary.Conv_VectorToTransform` (* (`KismetMathLibrary.Conv_IntVectorToVector` _array_element) (`self.Scale`))) false)))

(fn `UserConstructionScript`
  (`|ExecutionSequence`
    (:`then_0`
      ;[1 1 1] On click, get new seed
      (if (not (`self.NewSeed`))
        (set `self.NewSeed` false)
        (bind _output_get (set `self.Seed` (`KismetMathLibrary.RandomInteger` 900000)))
        (`KismetMathLibrary.SetRandomStreamSeed` (`self.Stream`) _output_get)))
    (:`then_1`
      ;[1 1 1] Manually set seed
      (`KismetMathLibrary.SetRandomStreamSeed` (`self.Stream`) (`self.Seed`)))
    (:`then_2`
      (`self.GenerateMap`))))